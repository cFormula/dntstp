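; An audio visualizer controller that turns a sound track into a field of height-animated cubes, like a graphic equalizer.
; BeginPlay starts the audio, spawns CubicEQ actors in a square-root-wide grid, then shuffles the array to scatter frequency bands across it.
; Each Tick samples the Track's spectrum at current game time, with one band per cube driving Z scale.
; Tick also continuously yaws its own root, to which the cubes are not attached.
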(event EventBeginPlay
  (Audio|Components|Audio|Play (Variables|Default|GetAudio) 0.0)
  (CallFunction|SpawnGrid)
  (Utilities|Array|Shuffle (Variables|Default|GetBPCubeArray)))

(event Collision|EventActorBeginOverlap
  (params (OtherActor :type Actor%20Object%20Reference)))

(event EventTick
  (params (DeltaSeconds :type Float%20%28single-precision%29))
  (Utilities|FlowControl|Sequence
    (:then_0
      (bind _outspectrum (Class|SoundVisualizationStatics|CalculateFrequencySpectrum (Variables|Default|GetTrack) 0 (Utilities|Time|GetGameTimeinSeconds) 0.1 (Utilities|Array|Length (Variables|Default|GetBPCubeArray))))
      (Variables|Default|SetSpectrum _outspectrum)
      (for (_array_element _array_index) (Variables|Default|GetBPCubeArray)
        (Transformation|SetActorScale3D _array_element (Math|Vector|MakeVector 1.0 1.0 (* (Math|Float|Absolute(Float) (Utilities|Array|Get(acopy) (Variables|Default|GetSpectrum) _array_index)) 0.1)))))
    (:then_1
      (Transformation|AddRelativeRotation (Variables|Default|GetDefaultSceneRoot) (Math|Rotator|MakeRotator 0.0 0.0 (* DeltaSeconds 9e+01)) false false))))

(fn ConstructionScript)

(fn SpawnGrid
  (bind _distance (Variables|Default|GetDistance))
  (for _index (range 0 (- (Variables|Default|GetNumberOfCubes) 1))
    (bind _returnvalue (Game|SpawnActorfromClass "/Game/Blueprints/Effects/CubicEQ.CubicEQ_C" (Math|Transform|MakeTransform (Math|Vector|MakeVector (* (Variables|Default|GetRow) _distance) (* (Variables|Default|GetColumn) _distance) 0.0) "0, 0, 0" "1,1,1") "AlwaysSpawn" 0 0))
    (Utilities|Array|Add (Variables|Default|GetBPCubeArray) _returnvalue)
    (Math|Integer|IncrementInt (Variables|Default|GetRow)
      (:%20%20
        (if (== (Variables|Default|GetRow) (Math|Float|Truncate (Math|Float|Sqrt (Math|Conversions|ToFloat(Integer) (Variables|Default|GetNumberOfCubes)))))
          (Math|Integer|IncrementInt (Variables|Default|GetColumn)
            (:%20%20
              (Variables|Default|SetRow 0))))))))
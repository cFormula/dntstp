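; Main player character Blueprint that moves by launching itself in short bursts rather than walking.
; Pressing W, A, S or D calls LaunchCharacter along the actor's forward or right vector at a fixed speed, overriding existing velocity on all axes.
; Turn and LookUp axes drive controller yaw and pitch for camera look.
; The Dashing event, tick and overlap events are empty stubs, and the construction script does nothing.
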(event Custom|Dashing
  (Utilities|FlowControl|Sequence
    (:then_0
      (if true
        _))))

(event Collision|EventActorBeginOverlap
  (params (OtherActor :type Actor%20Object%20Reference)))

(event EventTick
  (params (DeltaSeconds :type Float%20%28single-precision%29)))

(event Input|AxisEvents|InputAxisTurn
  (params (AxisValue :type Float%20%28single-precision%29))
  (Pawn|Input|AddControllerYawInput AxisValue))

(event Input|AxisEvents|InputAxisLookUp
  (params (AxisValue :type Float%20%28single-precision%29))
  (Pawn|Input|AddControllerPitchInput AxisValue))

(event Input|KeyboardEvents|D
  (params (Key :type Key%20Structure))
  (:Pressed
    (Character|LaunchCharacter (* (Transformation|GetActorRightVector) 2.5e+03) true true)))

(event Input|KeyboardEvents|W
  (params (Key :type Key%20Structure))
  (:Pressed
    (Character|LaunchCharacter (* (Transformation|GetActorForwardVector) 2.5e+03) true true)))

(event Input|KeyboardEvents|S
  (params (Key :type Key%20Structure))
  (:Pressed
    (Character|LaunchCharacter (* (Transformation|GetActorForwardVector) -2.5e+03) true true)))

(event Input|KeyboardEvents|A
  (params (Key :type Key%20Structure))
  (:Pressed
    (Character|LaunchCharacter (* (Transformation|GetActorRightVector) -2.5e+03) true true)))

(fn ConstructionScript)